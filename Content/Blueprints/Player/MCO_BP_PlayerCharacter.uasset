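; Player character Blueprint that handles interaction, pause and valuable-damage feedback.
; The E key calls a server interaction on the MCOInteraction component, and the Pause input action pushes the pause menu widget onto the UI menu layer through the player controller's HUD base.
; On BeginPlay it binds to the MCO event subsystem's valuable-damaged event and prints the damage value as on-screen text.
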(event `Key|E`
  (params (Key :type "Key Structure"))
  (:`Pressed`
    (`MCO_InteractionComponent.Server_DoInteraction` (`self.MCO_Interaction`))))

(event `EnhancedInput|/Game/Input/Actions/IA_Pause`
  (params (ActionValue :type Boolean) (ElapsedSeconds :type "Float (double-precision)") (TriggeredSeconds :type "Float (double-precision)") (InputAction :type "InputAction Object Reference" :default "/Game/Input/Actions/IA_Pause.IA_Pause"))
  (:`Started`
    (bind _asmoving_co_player_controller (cast `MovingCoPlayerController` (`self.GetController`)))
    (`MCO_HUDBase.PushWidgetToLayerStack` (`MovingCoPlayerController.GetHUDBase` _asmoving_co_player_controller) (struct :`TagName` "UI.Layer.Menu") "/Game/UI/Menus/MCO_WB_PauseMenu.MCO_WB_PauseMenu_C")))

(event `self.ReceiveBeginPlay`
  (add `MCO_AllEvents.OnValuableDamaged` (`MCO_EventSubsystem.GetAllEvents` (subsystem `MCO_EventSubsystem`)) (delegate `OnValuableDamaged`)))

(event `OnValuableDamaged`
  (params (ValueDamage :type "Float (single-precision)") (Location :type "Vector Structure (by ref)"))
  (`KismetSystemLibrary.PrintText` (`|FormatText` "Valuable damaged {x} pts" ValueDamage) true true (struct :`G` 0.66 :`B` 1.0 :`A` 1.0) 5.0))

(fn `UserConstructionScript`)